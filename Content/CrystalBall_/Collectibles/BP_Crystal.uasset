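; BP_Crystal is a collectible crystal that flies into the player and vanishes when the player pawn overlaps it.
; On overlap it stores its starting location, scale and light intensity, then plays the CrystalCollect timeline.
; Timeline tracks lerp it toward the player's current position, shrink it to zero and fade its point light, then the actor is destroyed.
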(event EventBeginPlay)

(event Collision|EventActorBeginOverlap
  (params (OtherActor :type Actor%20Object%20Reference))
  (if (== OtherActor (Game|Player|GetPlayerPawn 0))
    (CallFunction|StoreStartingValues)
    (bind (_direction _crystalcollection _lightintensity) (Timeline|CrystalCollect Play)
      (:Update
        (CallFunction|MovetoPlayer _crystalcollection)
        (CallFunction|ScaleCrystal _crystalcollection)
        (CallFunction|AdjustLight _lightintensity))
      (:Finished
        (Actor|DestroyActor)))))

(event EventTick
  (params (DeltaSeconds :type Float%20%28single-precision%29)))

(fn ConstructionScript)

(fn MovetoPlayer
  (params (Alpha :type Float%20%28single-precision%29))
  (Transformation|SetActorLocation (Math|Vector|Lerp(Vector) (Variables|Default|GetLerpStartLocation) (Transformation|GetActorLocation (Game|Player|GetPlayerPawn 0)) Alpha) false false))

(fn StoreStartingValues
  (Variables|Default|SetLerpStartLocation (Transformation|GetActorLocation))
  (Variables|Default|SetStartScale (Transformation|GetActorScale3D))
  (Variables|Default|SetStartLightIntensity (Variables|/Script/Engine.LightComponentBase|GetIntensity (Variables|Default|GetPointLight))))

(fn ScaleCrystal
  (params (Alpha :type Float%20%28single-precision%29))
  (Transformation|SetActorScale3D (Math|Vector|Lerp(Vector) (Variables|Default|GetStartScale) "0, 0, 0" Alpha)))

(fn AdjustLight
  (params (Alpha :type Float%20%28single-precision%29))
  (Rendering|Components|Light|SetIntensity (Variables|Default|GetPointLight) (Math|Float|Lerp (Variables|Default|GetStartLightIntensity) 0.0 Alpha)))